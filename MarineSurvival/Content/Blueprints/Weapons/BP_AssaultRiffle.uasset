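; Assault rifle child weapon Blueprint that provides automatic hitscan fire, setting its magazine size and sounds at construction.
; Firing checks that the Marine is alive, has ammo and is in an allowed state, then starts muzzle flash, loop sound and a repeating WeaponTrace timer.
; Each trace spends ammo, then applies damage and impact effects on a hit or draws a smoke trail on a miss.
; Stopping clears the effects and timer and plays an end sound.
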(event `self.ReceiveBeginPlay`
  (`parent.ReceiveBeginPlay`))

(fn `StartFiringWeapon`
  (bind _marine (`self.Marine`))
  (`parent.StartFiringWeapon`)
  (if (and (`/Game/Blueprints/Pawns/BP_Marine.Is Alive` _marine) (`self.HaveAmmo`) (`|EnumInequality` (`/Game/Blueprints/Pawns/BP_Marine.State` _marine) "NewEnumerator2"))
    (set `/Game/Blueprints/Pawns/BP_Marine.State` "NewEnumerator1" (`self.Marine`))
    (`ActorComponent.Activate` (`self.P_Weapon_MF`) false)
    (bind _returnvalue (`GameplayStatics.SpawnSound2D` (`self.FireSound`) 1.0 1.0 0.0 null))
    (set `self.WeaponFireSound` _returnvalue)
    (`self.WeaponTrace`)
    (`KismetSystemLibrary.K2_SetTimer` null "WeaponTrace" (`self.WeaponFireRate`) true)))

(fn `StopFiringWeapon`
  (bind _weaponfiresound (`self.WeaponFireSound`))
  (`parent.StopFiringWeapon`)
  (`ActorComponent.Deactivate` (`self.P_Weapon_MF`))
  (`/Engine/EditorBlueprintResources/StandardMacros.IsValid` _weaponfiresound
    (:`Is Valid`
      (`AudioComponent.Stop` _weaponfiresound)
      (`KismetSystemLibrary.K2_ClearTimer` null "WeaponTrace")
      (if (`/Game/Blueprints/Pawns/BP_Marine.Is Alive` (`self.Marine`))
        (`GameplayStatics.SpawnSound2D` "/Game/Sounds/Weapon_AssaultRifle/Stereo/RifleFireEnd_Cue.RifleFireEnd_Cue" 1.0 1.0 0.0 null)))))

(fn `UserConstructionScript`
  (`parent.UserConstructionScript`)
  (set `self.MaxAmmo` 30)
  (set `self.FireSound` "/Game/Sounds/Weapon_AssaultRifle/Stereo/RifleFireLoop_Cue.RifleFireLoop_Cue")
  (set `self.ReloadSound` "/Game/Sounds/Weapon_AssaultRifle/Stereo/Weapon_AssaultRifle_Reload02_Stereo.Weapon_AssaultRifle_Reload02_Stereo"))

(fn `WeaponTrace`
  (bind (_returnvalue_location _returnvalue_rotation _returnvalue_scale) (`KismetMathLibrary.BreakTransform` (`SceneComponent.GetSocketTransform` (`self.Weapon`) "MuzzleFlashSocket" "RTS_World")))
  (`parent.WeaponTrace`)
  (if (`self.HaveAmmo`)
    (bind _outhit (`KismetSystemLibrary.LineTraceSingle` (`self.GetWeaponTraceStart`) (`self.GetWeaponTraceEnd`) "TraceTypeQuery1"))
    (`/Engine/EditorBlueprintResources/StandardMacros.DecrementInt` (`self.CurrentAmmo`)
      (:`  `
        (bind (_bblockinghit _binitialoverlap _time _distance _location _impactpoint _normal _impactnormal _physmat _hitactor) (`GameplayStatics.BreakHitResult` _outhit))
        (if _bblockinghit
          (`GameplayStatics.ApplyDamage` _hitactor (`self.DamagePerShot`))
          (`self.SpawnImpactHit` _location)
          (else
            (bind _returnvalue (`GameplayStatics.SpawnEmitterAtLocation` "/Game/Particles/P_SmokeTrail.P_SmokeTrail" _returnvalue_location _returnvalue_rotation _returnvalue_scale))
            (`FXSystemComponent.SetVectorParameter` _returnvalue "Target" (`self.GetWeaponTraceEnd`))))))))