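; Base-style weapon Blueprint for the Marine that attaches to the character's WeaponPoint socket and manages ammo.
; WeaponTrace handles only an empty magazine, setting the Marine's state, playing a reload sound and refilling via a one-second timer.
; Helpers compute a muzzle-to-control-rotation trace segment, spawn smoke-trail and impact particles, and toggle weapon components.
; Start and stop firing are empty stubs, and no line trace is performed here.
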(event `self.ReceiveBeginPlay`
  (`self.K2_AttachToComponent` (`Character.Mesh` (`self.Marine`)) "WeaponPoint" "KeepWorld" "KeepWorld" "KeepRelative")
  (set `self.CurrentAmmo` (`self.MaxAmmo`)))

(fn `Activate`
  (`ActorComponent.Activate` (`self.Weapon`) false)
  (`ActorComponent.Activate` (`self.P_Weapon_MF`) false))

(fn `Deactivate`
  (`ActorComponent.Deactivate` (`self.Weapon`))
  (`ActorComponent.Deactivate` (`self.P_Weapon_MF`)))

(fn `GetWeaponTraceEnd`
  (returns (ReturnValue :type "Vector Structure"))
  (return (+ (`self.GetWeaponTraceStart`) (* (`KismetMathLibrary.GetForwardVector` (`Pawn.GetControlRotation` (`self.Marine`))) (`self.WeaponRange`)))))

(fn `GetWeaponTraceStart`
  (returns (ReturnValue :type "Vector Structure"))
  (return (`SceneComponent.GetSocketLocation` (`self.Weapon`) "MuzzleFlash")))

(fn `HaveAmmo`
  (returns (ReturnValue :type Boolean))
  (return (> (`self.CurrentAmmo`) 0)))

(fn `SpawnImpactHit`
  (params (HitLocation :type "Vector Structure"))
  (bind (_returnvalue_location _returnvalue_rotation _returnvalue_scale) (`KismetMathLibrary.BreakTransform` (`SceneComponent.GetSocketTransform` (`self.Weapon`) "MuzzleFlashSocket" "RTS_World")))
  (bind _returnvalue (`GameplayStatics.SpawnEmitterAtLocation` "/Game/Particles/P_SmokeTrail.P_SmokeTrail" _returnvalue_location _returnvalue_rotation _returnvalue_scale))
  (`FXSystemComponent.SetVectorParameter` _returnvalue "Target" HitLocation)
  (`GameplayStatics.SpawnEmitterAtLocation` "/Game/Effects/Weapons/Impacts/P_AssaultRifle_IH.P_AssaultRifle_IH" HitLocation))

(fn `StartFiringWeapon`)

(fn `StopFiringWeapon`)

(fn `UserConstructionScript`)

(fn `WeaponReload`
  (set `self.CurrentAmmo` (`self.MaxAmmo`))
  (set `/Game/Blueprints/Pawns/BP_Marine.State` "NewEnumerator0" (`self.Marine`)))

(fn `WeaponTrace`
  (if (`self.HaveAmmo`)
    _
    (elif (`|EnumInequality` (`/Game/Blueprints/Pawns/BP_Marine.State` (`self.Marine`)) "NewEnumerator2")
      (set `/Game/Blueprints/Pawns/BP_Marine.State` "NewEnumerator2" (`self.Marine`))
      (`self.StopFiringWeapon`)
      (`GameplayStatics.SpawnSound2D` (`self.ReloadSound`) 1.0 1.0 0.0 null)
      (`KismetSystemLibrary.K2_SetTimer` null "WeaponReload" 1.0))))