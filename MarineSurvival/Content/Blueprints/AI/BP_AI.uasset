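; BP_AI is an alien enemy character with health and death handling for the Mars Marine game.
; DecreaseHealth subtracts damage from a clamped Health value and returns it, without triggering death itself.
; KillAI flags the alien dead, shuts off movement and collision, increments the BP_Marine player's kills and registers the death with BP_MarsMarine_GameMode.
; The event graph holds only disabled placeholder events.
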(fn `DecreaseHealth`
  (params (Damage :type "Float (double-precision)"))
  (returns (Health :type "Float (double-precision)"))
  (bind _output_get (set `self.Health` (`KismetMathLibrary.FClamp` (- (`self.Health`) Damage) 0.0 100.0)))
  (return _output_get))

(fn `KillAI`
  (bind _charactermovement (`self.CharacterMovement`))
  (set `self.Dead` true)
  (`MovementComponent.StopMovementImmediately` _charactermovement)
  (`ActorComponent.Deactivate` _charactermovement)
  (`self.SetActorEnableCollision` false)
  (bind _asbp_marine (cast `/Game/Blueprints/Pawns/BP_Marine` (`GameplayStatics.GetPlayerCharacter` 0)))
  (`/Game/Blueprints/Pawns/BP_Marine.Increase Kills` _asbp_marine)
  (bind _asbp_mars_marine_game_mode (cast `/Game/Blueprints/GameMode/BP_MarsMarine_GameMode` (`GameplayStatics.GetGameMode`)))
  (`/Game/Blueprints/GameMode/BP_MarsMarine_GameMode.Register Alien Death` _asbp_mars_marine_game_mode self))

(fn `UserConstructionScript`)