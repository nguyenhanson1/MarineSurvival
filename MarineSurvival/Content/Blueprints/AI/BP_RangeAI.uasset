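; BP_RangeAI is a ranged enemy AI that turns to face the player's BP_Marine every tick and shoots at it.
; When PawnSensing sees the marine, it fires a debug line trace, whose result is unused, and spawns BP_EnemyBullet at the weapon socket.
; Damage lowers clamped health, but the zero-health branch is empty.
; KillAI, which disables collision and increments the marine's kills, is not called here.
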(event `self.ReceiveTick`
  (params (DeltaSeconds :type "Float (single-precision)"))
  (bind _asbp_marine (cast `/Game/Blueprints/Pawns/BP_Marine` (`GameplayStatics.GetPlayerCharacter` 0)))
  (bind (_returnvalue_roll _returnvalue_pitch _returnvalue_yaw) (`KismetMathLibrary.BreakRotator` (`KismetMathLibrary.FindLookAtRotation` (`self.K2_GetActorLocation`) (`self.K2_GetActorLocation` _asbp_marine))))
  (`self.K2_SetActorRotation` (`KismetMathLibrary.MakeRotator` _returnvalue_roll _returnvalue_pitch _returnvalue_yaw)))

(event `self.PawnSensing.OnSeePawn`
  (params (Pawn :type "Pawn Object Reference"))
  (bind _returnvalue (`self.K2_GetActorLocation`))
  (cast `/Game/Blueprints/Pawns/BP_Marine` Pawn)
  (`KismetSystemLibrary.LineTraceSingle` :`Start` _returnvalue :`End` (+ _returnvalue (* (`KismetMathLibrary.GetForwardVector` (`self.GetControlRotation`)) 1000.0)) :`TraceChannel` "TraceTypeQuery1" :`DrawDebugType` "ForDuration" :`DrawTime` 1.0)
  (`|SpawnActorFromClass` "/Game/Blueprints/AI/BP_EnemyBullet.BP_EnemyBullet_C" (`SceneComponent.GetSocketTransform` (`self.Mesh`) "WeaponSocket" "RTS_World") "Undefined" "OverrideRootScale" self null))

(event `self.ReceiveAnyDamage`
  (params (Damage :type "Float (single-precision)") (DamageType :type "DamageType Object Reference") (InstigatedBy :type "Controller Object Reference") (DamageCauser :type "Actor Object Reference"))
  (if true
    (bind _health (`self.DecreaseHealth` Damage))
    (if (== _health 0.0)
      _)))

(fn `DecreaseHealth`
  (params (Damage :type "Float (double-precision)"))
  (returns (Health :type "Float (double-precision)"))
  (bind _output_get (set `self.Health` (`KismetMathLibrary.FClamp` (- (`self.Health`) Damage) 0.0 100.0)))
  (return _output_get))

(fn `KillAI`
  (set `self.Dead` true)
  (`self.SetActorEnableCollision` false)
  (bind _asbp_marine (cast `/Game/Blueprints/Pawns/BP_Marine` (`GameplayStatics.GetPlayerCharacter` 0)))
  (`/Game/Blueprints/Pawns/BP_Marine.Increase Kills` _asbp_marine)
  (cast `/Game/Blueprints/GameMode/BP_MarsMarine_GameMode` (`GameplayStatics.GetGameMode`)))

(fn `UserConstructionScript`)