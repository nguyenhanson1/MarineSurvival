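; BP_EnemyBullet is an enemy projectile that damages BP_Marine actors on contact.
; Each tick it moves with a swept local offset built from its world forward vector, scaled by Speed and delta time.
; When its Sphere overlaps a Marine it applies fixed damage and destroys itself, ignoring other actor types.
; A timer set on BeginPlay calls Destroy to limit its lifetime to a few seconds.
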(event `self.ReceiveBeginPlay`
  (`KismetSystemLibrary.K2_SetTimer` null "Destroy" 3.0))

(event `self.ReceiveTick`
  (params (DeltaSeconds :type "Float (single-precision)"))
  (`self.K2_AddActorLocalOffset` (* (`self.GetActorForwardVector`) (* DeltaSeconds (`self.Speed`))) true))

(event `self.Sphere.OnComponentBeginOverlap`
  (params (OverlappedComponent :type "PrimitiveComponent Object Reference") (OtherActor :type "Actor Object Reference") (OtherComp :type "PrimitiveComponent Object Reference") (OtherBodyIndex :type Integer) (bFromSweep :type Boolean) (SweepResult :type "HitResult Structure (by ref)"))
  (bind _asbp_marine (cast `/Game/Blueprints/Pawns/BP_Marine` OtherActor))
  (`GameplayStatics.ApplyDamage` _asbp_marine 20.0 null null "/Script/Engine.DamageType")
  (`self.K2_DestroyActor`))

(fn `Destroy`
  (`self.K2_DestroyActor`))

(fn `UserConstructionScript`)